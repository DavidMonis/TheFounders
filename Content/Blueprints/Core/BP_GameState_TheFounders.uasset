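; Game state for The Founders that holds the resource economy of Brick, Iron, Wheat, Wool and Gold.
; BeginPlay creates the HUD widget with a reference to this state, sets game-and-UI input and starts a fast looping timer.
; An update function adds each resource's modifier and advances Time, granting Gold through a randomized modulo check scaled by GoldModifier.
; A separate function simply increments Gold.
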(event `self.ReceiveBeginPlay`
  (bind _returnvalue (`GameplayStatics.GetPlayerController` 0))
  (bind _returnvalue_2 (`|CreateWidget` "/Game/UI/W_HUD.W_HUD_C" _returnvalue self))
  (`UserWidget.AddToViewport` _returnvalue_2 0)
  (`WidgetBlueprintLibrary.SetInputMode_GameAndUIEx` _returnvalue _returnvalue_2 "DoNotLock" false)
  (`KismetSystemLibrary.K2_SetTimerDelegate` (`|CreateDelegate` :!event `BP_GameState_TheFounders_AutoGenFunc`) 0.1 true))

(fn `BP_GameState_TheFounders_AutoGenFunc`
  (bind _goldmodifier (`self.GoldModifier`))
  (set `self.Brick` (+ (`self.Brick`) (`self.BrickModifier`)))
  (set `self.Iron` (+ (`self.Iron`) (`self.IronModifier`)))
  (set `self.Wheat` (+ (`self.Wheat`) (`self.WheatModifier`)))
  (set `self.Wool` (+ (`self.Wool`) (`self.WoolModifier`)))
  (set `self.Time` (+ (`self.Time`) 1))
  (if (and (!= _goldmodifier 0) (== (mod (`self.Time`) (`KismetMathLibrary.RandomInteger` (/ 60 _goldmodifier))) 0))
    (set `self.Gold` (+ (`self.Gold`) 1))))

(fn `BP_GameState_TheFounders_AutoGenFunc1`
  (set `self.Gold` (+ (`self.Gold`) 1)))

(fn `UserConstructionScript`)